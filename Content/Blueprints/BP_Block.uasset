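; BP_Block is a block Blueprint that exposes a set of player-style interaction functions but contains no behavior of its own.
; Click, Grab, Push, their release counterparts, Interact and Place each take an Owner and return immediately as empty stubs.
; The event graph and construction script are also empty, with only disabled default event nodes.
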(fn `Click`
  (params (Owner :type "Actor Object Reference"))
  (returns (SelfCopy :type "Actor Object Reference"))
  (return null))

(fn `ClickRelease`
  (params (Owner :type "Actor Object Reference"))
  (returns (SelfCopy :type "Actor Object Reference"))
  (return null))

(fn `Grab`
  (params (Owner :type "Actor Object Reference"))
  (returns (SelfCopy :type "Actor Object Reference"))
  (return null))

(fn `GrabRelease`
  (params (Owner :type "Actor Object Reference"))
  (returns (SelfCopy :type "Actor Object Reference"))
  (return null))

(fn `Interact`
  (params (Owner :type "Actor Object Reference"))
  (returns (SelfCopy :type "Actor Object Reference"))
  (return null))

(fn `Place`
  (params (Owner :type "Actor Object Reference"))
  (returns (SelfCopy :type "Actor Object Reference"))
  (return null))

(fn `Push`
  (params (Owner :type "Actor Object Reference"))
  (returns (SelfCopy :type "Actor Object Reference"))
  (return null))

(fn `PushRelease`
  (params (Owner :type "Actor Object Reference"))
  (returns (SelfCopy :type "Actor Object Reference"))
  (return null))

(fn `UserConstructionScript`)