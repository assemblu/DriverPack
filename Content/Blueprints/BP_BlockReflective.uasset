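; BP_BlockReflective is a block Blueprint with no active logic of its own; its name suggests a reflective variant.
; Its interact, stop-interact and look-at overrides are inert, returning false or an empty message.
; The event graph holds only disabled default events, and the construction script just calls the parent, so any reflective behavior is defined outside these graphs.
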(fn `InteractWithInternal`
  (params (Interactor :type "Actor Object Reference") (HitComponent :type "PrimitiveComponent Object Reference"))
  (returns (Ack :type Boolean))
  (return false))

(fn `LookAtInternal`
  (params (Interactor :type "/Game/Blueprints/BP_ThirdPersonCharacter Object Reference") (Controller :type "PlayerController Object Reference") (HitComponent :type "PrimitiveComponent Object Reference"))
  (returns (LookAtActor :type "Actor Object Reference") (LookAtComponent :type "PrimitiveComponent Object Reference") (Message :type Text))
  (return null null ""))

(fn `StopInteractWithInternal`
  (params (Interactor :type "Actor Object Reference") (HitComponent :type "PrimitiveComponent Object Reference"))
  (returns (Ack :type Boolean))
  (return false))

(fn `UserConstructionScript`
  (`parent.UserConstructionScript`))