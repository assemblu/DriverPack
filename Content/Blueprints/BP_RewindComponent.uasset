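; Actor component for a time-rewind mechanic that records its owner's location history; the rewind playback itself is still empty.
; BeginPlay fills a fixed-length array with the starting location, then Tick overwrites it as a circular buffer, spending one frame on each index reset.
; Holding R sets a rewind flag that pauses recording.
; Debug prints show the first stored location and each buffer wrap, and only location is recorded.
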(event `self.ReceiveBeginPlay`
  (set `self.Owner` (`self.GetOwner`))
  (while (< (`self.StateInsertIndex`) (`self.StateLen`))
    (`KismetArrayLibrary.Array_Add` (`self.LocationState`) (`Actor.K2_GetActorLocation` (`self.Owner`)))
    (set `self.StateInsertIndex` (+ (`self.StateInsertIndex`) 1))))

(event `Key|R`
  (params (Key :type "Key Structure"))
  (:`Pressed`
    (set `self.IsRewinding` true))
  (:`Released`
    (set `self.IsRewinding` false)))

(event `self.ReceiveTick`
  (params (DeltaSeconds :type "Float (single-precision)"))
  (bind (_returnvalue_x _returnvalue_y _returnvalue_z) (`KismetMathLibrary.BreakVector` (`Actor.K2_GetActorLocation` (`self.Owner`))))
  (`|ExecutionSequence`
    (:`then_0`
      (if (not (`self.IsRewinding`))
        (if (< (`self.StateInsertIndex`) (`self.StateLen`))
          (`KismetMathLibrary.Vector_Set` (`|GetArrayItem` (`self.LocationState`) (`self.StateInsertIndex`)) _returnvalue_x _returnvalue_y _returnvalue_z)
          (set `self.StateInsertIndex` (+ (`self.StateInsertIndex`) 1))
          (else
            (set `self.StateInsertIndex` 0)
            (`KismetSystemLibrary.PrintString` "RESET State Insert Index" true true (struct :`R` 1.0 :`B` 0.074582 :`A` 1.0) 0.5 "1")))))
    (:`then_1`
      (if (`self.IsRewinding`)
        _))
    (:`then_2`
      (`KismetSystemLibrary.PrintString` (`KismetStringLibrary.Conv_VectorToString` (`|GetArrayItem` (`self.LocationState`))) true true (struct :`G` 0.66 :`B` 1.0 :`A` 1.0) 0.5 "0"))))